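; AI controller for the soldier enemy that runs BT_Soldat and caches the player character and controlled pawn on BeginPlay.
; Every Tick, it line traces from the pawn toward the player's mesh and writes whether the player is hit to a Blackboard bool.
; Custom events forward closeness, sight, random animation and player-death states to the soldier's AB_Comportement anim instance.
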(event Custom|IsClose
  (params (IsClose :type Boolean))
  (bind _asbp_soldat (Utilities|Casting|CastToBP_Soldat (Variables|Default|GetPawnControlled)))
  (bind _asab_comportement (Utilities|Casting|CastToAB_Comportement (Components|SkeletalMesh|GetAnimInstance (Variables|/Script/Engine.Character|GetMesh _asbp_soldat))))
  (Variables|/Game/Animation/AB_Comportement.AB_Comportement_C|SetIsClose _asab_comportement IsClose))

(event Custom|IsSeeing
  (params (IsSeeing :type Boolean))
  (bind _asbp_soldat (Utilities|Casting|CastToBP_Soldat (Variables|Default|GetPawnControlled)))
  (bind _asab_comportement (Utilities|Casting|CastToAB_Comportement (Components|SkeletalMesh|GetAnimInstance (Variables|/Script/Engine.Character|GetMesh _asbp_soldat))))
  (Variables|/Game/Animation/AB_Comportement.AB_Comportement_C|SetIsSeeing _asab_comportement IsSeeing))

(event Custom|RandomAnim
  (params (RandomAnim :type Boolean))
  (bind _asbp_soldat (Utilities|Casting|CastToBP_Soldat (Variables|Default|GetPawnControlled)))
  (bind _asab_comportement (Utilities|Casting|CastToAB_Comportement (Components|SkeletalMesh|GetAnimInstance (Variables|/Script/Engine.Character|GetMesh _asbp_soldat))))
  (Variables|/Game/Animation/AB_Comportement.AB_Comportement_C|SetRandomAnim _asab_comportement RandomAnim))

(event Custom|PlayerIsDead
  (params (IsPlayerDead :type Boolean))
  (bind _asbp_soldat (Utilities|Casting|CastToBP_Soldat (Variables|Default|GetPawnControlled)))
  (bind _asab_comportement (Utilities|Casting|CastToAB_Comportement (Components|SkeletalMesh|GetAnimInstance (Variables|/Script/Engine.Character|GetMesh _asbp_soldat))))
  (Variables|/Game/Animation/AB_Comportement.AB_Comportement_C|SetPlayerIsDead _asab_comportement IsPlayerDead))

(event EventBeginPlay
  (AI|RunBehaviorTree "/Game/Blueprints/BT_Soldat.BT_Soldat")
  (Utilities|FlowControl|DelayUntilNextTick)
  (bind _asbp_third_person_character (Utilities|Casting|CastToBP_ThirdPersonCharacter (Game|GetPlayerCharacter 0)))
  (Variables|Default|SetPlayer _asbp_third_person_character)
  (Variables|Default|SetPawnControlled (Pawn|GetControlledPawn)))

(event EventTick
  (params (DeltaSeconds :type Float%20%28single-precision%29))
  (bind _pawncontrolled (Variables|Default|GetPawnControlled))
  (bind _returnvalue (Transformation|GetActorLocation _pawncontrolled))
  (bind _outhit (Collision|LineTraceByChannel _returnvalue (+ _returnvalue (* (Math|Vector|Normalize (- (Transformation|GetWorldLocation (Variables|/Script/Engine.Character|GetMesh (Variables|Default|GetPlayer))) (Transformation|GetActorLocation (Variables|Default|GetPawnControlled)))) (Variables|Default|GetDistance))) "TraceTypeQuery1" false 0 "None"))
  (Utilities|Casting|CastToBP_ThirdPersonCharacter (.HitActor (Collision|BreakHitResult _outhit))
    (:then
      (AI|Components|Blackboard|SetValueasBool (AI|GetBlackboard 0) (Variables|Default|GetBB_Key_PlayerName) true))
    (:CastFailed
      (AI|Components|Blackboard|SetValueasBool (AI|GetBlackboard 0) (Variables|Default|GetBB_Key_PlayerName) false))))

(fn ConstructionScript)